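; BP_WallSconce is a wall lamp with a configurable cone light that can be switched, recolored or destroyed by an EMP.
; The construction script applies brightness, color, cone angles and on/off state to SconceLight.
; UpdateLight stores and applies visibility, with TurnOff forcing it off, while two functions temporarily override or restore the configured color.
; EMPDestroy spawns an explosion at the lamp mesh and destroys the actor.
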(event `/Game/Skvt/Blueprints/BPI_ElectricDevice.TurnOff`
  (`self.UpdateLight` false))

(event `/Game/Skvt/Blueprints/BPI_ElectricDevice.EMPDestroy`
  (`GameplayStatics.SpawnEmitterAtLocation` "/Game/StarterContent/Particles/P_Explosion.P_Explosion" (`SceneComponent.K2_GetComponentLocation` (`self.SM_Lamp_Wall`)))
  (`self.K2_DestroyActor`))

(fn `Change Light Color`
  (params (`New Color` :type "LinearColor Structure"))
  (`LightComponent.SetLightColor` (`self.SconceLight`) `New Color` true))

(fn `Restore Light Color`
  (`LightComponent.SetLightColor` (`self.SconceLight`) (`self.Color`) true))

(fn `UpdateLight`
  (params (IsOnLocal :type Boolean))
  (bind _output_get (set `self.IsOn` IsOnLocal))
  (`SceneComponent.SetVisibility` (`self.SconceLight`) _output_get false))

(fn `UserConstructionScript`
  (bind _sconcelight (`self.SconceLight`))
  (`LightComponent.SetIntensity` _sconcelight (`self.Brightness`))
  (`LightComponent.SetLightColor` _sconcelight (`self.Color`) true)
  (`SpotLightComponent.SetInnerConeAngle` _sconcelight (`self.Inner Cone Angle`))
  (`SpotLightComponent.SetOuterConeAngle` _sconcelight (`self.Outer Cone Angle`))
  (`SceneComponent.SetVisibility` _sconcelight (`self.IsOn`) false))