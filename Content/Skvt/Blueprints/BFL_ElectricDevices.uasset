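; Blueprint function library for finding electric devices near a given actor.
; GetElectricDevicesInDistance gathers every world actor implementing BPI_ElectricDevice and returns those within a maximum distance of the origin actor.
; The IsInRange helper performs the inclusive distance check between a location and each actor's location.
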(fn `Get Electric Devices In Distance`
  (params (`Max Distance` :type "Float (double-precision)") (`Origin Actor` :type "Actor Object Reference"))
  (returns (`Selected Devices` :type "Array of Actor Object Reference"))
  (locals (Devices :type "Array of Actor Object Reference"))
  (set `local.Devices` (`|MakeArray` null :!type "Actor Object Reference"))
  (bind _outactors (`GameplayStatics.GetAllActorsWithInterface` null "/Game/Skvt/Blueprints/BPI_ElectricDevice.BPI_ElectricDevice_C"))
  (for _array_element _outactors
    (if (`self.Is in Range` `Max Distance` (`Actor.K2_GetActorLocation` `Origin Actor`) _array_element)
      (`KismetArrayLibrary.Array_Add` (`local.Devices`) _array_element)))
  (return (`local.Devices`)))

(fn `Is in Range`
  (params (Distance :type "Float (double-precision)") (OriginLocation :type "Vector Structure") (Actor :type "Actor Object Reference"))
  (returns (IsTrue :type Boolean))
  (return (>= Distance (`KismetMathLibrary.Vector_Distance` OriginLocation (`Actor.K2_GetActorLocation` Actor)))))